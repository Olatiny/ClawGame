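; BP_Claw is a player-driven claw that moves horizontally, then lowers to pick up and drop actors.
; Pressing OctoAction releases a held actor or starts descending; releasing it raises the claw and line-traces below, ignoring BP_Floor, to grab.
; Tick lerps height toward the start Z or a short downward trace's impact, and pins the grabbed actor underneath with collision and physics off.
; Loop-based OctoAction, Ascend and Decend functions are never called here.
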(event `InputAction|OctoAction`
  (params (Key :type "Key Structure"))
  (bind (_returnvalue_x _returnvalue_y _returnvalue_z) (`KismetMathLibrary.BreakVector` (`self.K2_GetActorLocation`)))
  (bind _grabbedactor (`self.GrabbedActor`))
  (:`Pressed`
    (if (`self.Holding`)
      (set `self.Holding` false)
      (`self.SetActorEnableCollision` _grabbedactor true)
      (`PrimitiveComponent.SetSimulatePhysics` (`|GetArrayItem` (`self.K2_GetComponentsByClass` _grabbedactor "/Script/Engine.PrimitiveComponent")) true)
      (else
        (set `self.GoingUp?` false))))
  (:`Released`
    (set `self.GoingUp?` true)
    (bind _outactors (`GameplayStatics.GetAllActorsOfClass` "/Game/Characters/BP_Floor.BP_Floor_C"))
    (bind (_outhit _returnvalue) (`KismetSystemLibrary.LineTraceSingle` (`self.K2_GetActorLocation`) (`KismetMathLibrary.MakeVector` _returnvalue_x _returnvalue_y (- _returnvalue_z 50.0)) "TraceTypeQuery1" false _outactors))
    (if _returnvalue
      (bind _output_get (set `self.GrabbedActor` (`.HitActor` (`GameplayStatics.BreakHitResult` _outhit))))
      (`self.SetActorEnableCollision` _output_get false)
      (`PrimitiveComponent.SetSimulatePhysics` (`|GetArrayItem` (`self.K2_GetComponentsByClass` _output_get "/Script/Engine.PrimitiveComponent")) false)
      (set `self.Holding` true)
      (`KismetSystemLibrary.PrintString` "Grabbed"))))

(event `self.ReceiveBeginPlay`
  (bind (_returnvalue_x _returnvalue_y _returnvalue_z) (`KismetMathLibrary.BreakVector` (`self.K2_GetActorLocation`)))
  (set `self.ZTop` _returnvalue_z))

(event `InputAxis|MoveHorizontal`
  (params (AxisValue :type "Float (single-precision)"))
  ;[1 1 1] Horizontal Movement
  (if (not (`self.Decending/Acending`))
    (`self.K2_AddActorWorldOffset` (`KismetMathLibrary.MakeVector` 0.0 (* AxisValue (`self.Speed`))) true)))

(event `InputAxis|MoveVertical`
  (params (AxisValue :type "Float (single-precision)"))
  ;[1 1 1] Vertical Movement
  (if (not (`self.Decending/Acending`))
    (`self.K2_AddActorWorldOffset` (`KismetMathLibrary.MakeVector` (* AxisValue (`self.Speed`))) true)))

(event `self.ReceiveTick`
  (params (DeltaSeconds :type "Float (single-precision)"))
  (bind (_returnvalue_x _returnvalue_y _returnvalue_z) (`KismetMathLibrary.BreakVector` (`self.K2_GetActorLocation`)))
  (bind (_returnvalue_x_2 _returnvalue_y_2 _returnvalue_z_2) (`KismetMathLibrary.BreakVector` (`self.K2_GetActorLocation`)))
  (bind (_returnvalue_x_3 _returnvalue_y_3 _returnvalue_z_3) (`KismetMathLibrary.BreakVector` (`self.K2_GetActorLocation`)))
  (bind _lerpalpha (`self.LerpAlpha`))
  (set `self.Delta Seconds` DeltaSeconds)
  (if (`self.Holding`)
    (`self.K2_SetActorLocation` (`self.GrabbedActor`) (`KismetMathLibrary.MakeVector` _returnvalue_x_2 _returnvalue_y_2 (- _returnvalue_z_2 200.0)) false false))
  (if (`self.GoingUp?`)
    (`self.K2_SetActorLocation` (`KismetMathLibrary.MakeVector` _returnvalue_x _returnvalue_y (`KismetMathLibrary.Lerp` _returnvalue_z (`self.ZTop`) _lerpalpha)))
    (else
      (bind _outhit (`KismetSystemLibrary.LineTraceSingle` (`self.K2_GetActorLocation`) (`KismetMathLibrary.MakeVector` _returnvalue_x_3 _returnvalue_y_3 (- _returnvalue_z_3 5.0)) "TraceTypeQuery1"))
      (`self.K2_SetActorLocation` (`KismetMathLibrary.MakeVector` _returnvalue_x_3 _returnvalue_y_3 (`KismetMathLibrary.Lerp` _returnvalue_z_3 (.z (`.ImpactPoint` (`GameplayStatics.BreakHitResult` _outhit))) _lerpalpha))))))

(fn `Ascend`
  (while (>= (`self.ZTop`) (.z (`self.K2_GetActorLocation`)))
    (`self.K2_AddActorWorldOffset` (`KismetMathLibrary.MakeVector` 0.0 0.0 (* 1.0 (`self.ZSpeed`))) true))
  (set `self.Decending/Acending` false))

(fn `Decend`
  (set `self.Decending/Acending` true)
  (while (== (`KismetArrayLibrary.Array_Length` (`self.GetOverlappingActors` null)) 0)
    (`self.K2_AddActorWorldOffset` (`KismetMathLibrary.MakeVector` 0.0 0.0 (* -1.0 (`self.ZSpeed`))) true))
  (set `self.Decending/Acending` false))

(fn `HandleHit`)

(fn `Octo Action`
  (set `self.Decending/Acending` true))

(fn `UserConstructionScript`)