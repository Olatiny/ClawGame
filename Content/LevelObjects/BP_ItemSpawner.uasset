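; BP_ItemSpawner is a level object that spawns a random item class from ItemsToSpawn at its own location and rotation every second.
; BeginPlay loops through SpawnItem and a one-second Delay indefinitely, storing only the newest actor in CurrentItem without removing earlier ones.
; SpawnItem also prints a random index, drawn separately from the one used to spawn.
; AttemptToSpawn is an empty stub.
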(event `self.ReceiveBeginPlay`
  (`self.SpawnItem` :!label _label)
  (`KismetSystemLibrary.Delay` 1.0)
  (goto _label))

(fn `AttemptToSpawn`)

(fn `SpawnItem`
  (bind _returnvalue (`KismetMathLibrary.RandomIntegerInRange` 0 (`KismetArrayLibrary.Array_LastIndex` (`self.ItemsToSpawn`))))
  (`KismetSystemLibrary.PrintString` (`KismetStringLibrary.Conv_IntToString` _returnvalue))
  (bind _returnvalue_2 (`|SpawnActorFromClass` (`|GetArrayItem` (`self.ItemsToSpawn`) _returnvalue) (`KismetMathLibrary.MakeTransform` (`self.K2_GetActorLocation`) (`self.K2_GetActorRotation`)) "AdjustIfPossibleButAlwaysSpawn" "MultiplyWithRoot" null null))
  (set `self.CurrentItem` _returnvalue_2))

(fn `UserConstructionScript`)