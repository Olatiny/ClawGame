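; BP_TimeBasedItemSpawner is a level object that keeps spawning random items at its own location.
; On BeginPlay it loops endlessly, calling SpawnItem and then waiting DelayTime.
; SpawnItem picks a random class from ItemsToSpawn, spawns it with the spawner's rotation, adjusting for collisions, and stores it in CurrentItem.
; Earlier items are never checked or removed, and AttemptToSpawn is an empty stub.
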(event `self.ReceiveBeginPlay`
  (`self.SpawnItem` :!label _label)
  (`KismetSystemLibrary.Delay` (`self.DelayTime`))
  (goto _label))

(fn `AttemptToSpawn`)

(fn `SpawnItem`
  (bind _returnvalue (`|SpawnActorFromClass` (`|GetArrayItem` (`self.ItemsToSpawn`) (`KismetMathLibrary.RandomIntegerInRange` 0 (`KismetArrayLibrary.Array_LastIndex` (`self.ItemsToSpawn`)))) (`KismetMathLibrary.MakeTransform` (`self.K2_GetActorLocation`) (`self.K2_GetActorRotation`)) "AdjustIfPossibleButAlwaysSpawn" "MultiplyWithRoot" null null))
  (set `self.CurrentItem` _returnvalue))

(fn `UserConstructionScript`)